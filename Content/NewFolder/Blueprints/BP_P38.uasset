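; BP_P38 is an aircraft actor, apparently a P-38, that spins its two propellers while drifting at constant speed along world X.
; Each Tick passes the right and left propeller components to PropellerRotation, which adds local roll from RotationRate and delta time.
; Tick then applies a delta-time-scaled world offset, so movement is frame-rate independent and ignores the plane's facing.
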(event EventBeginPlay)

(event Collision|EventActorBeginOverlap
  (params (OtherActor :type Actor%20Object%20Reference)))

(event EventTick
  (params (DeltaSeconds :type Float%20%28single-precision%29))
  (CallFunction|PropellerRotation (Variables|Default|GetR.Properller))
  (CallFunction|PropellerRotation (Variables|Default|GetL.Propeller))
  (Transformation|AddActorWorldOffset (Math|Vector|MakeVector (* (Utilities|Time|GetWorldDeltaSeconds) 6e+01) 0.0 0.0)))

(fn ConstructionScript)

(fn PropellerRotation
  (params (self2 :type Scene%20Component%20Object%20Reference))
  (Transformation|AddLocalRotation self2 (Math|Rotator|MakeRotator (* (Utilities|Time|GetWorldDeltaSeconds) (Variables|Default|GetRotationRate)) 0.0 0.0) false false))